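; Interactable main table that lets the player sit at it or teleport to a GodDesk.
; Box overlap enables input, shows a SwitchCharacterWidget and opens a gate for the E key.
; E runs a timeline that lerps the player's transform and control rotation to the seat point, setting IsSit and a looping crouch idle animation.
; Q clears the seated state and restores Animation Blueprint mode, while C teleports the player.
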(event `Key|E`
  (params (Key :type "Key Structure"))
  (bind _returnvalue (`GameplayStatics.GetPlayerController` 0))
  (:`Pressed`
    (if (not (`/Game/Blueprints/BP_player.IsSit` (stale `self.Box.OnComponentBeginOverlap` _asbp_player)))
      (`/Engine/EditorBlueprintResources/StandardMacros.Gate` true :!label _label
        (:`Exit`
          (bind _capsulecomponent (`Character.CapsuleComponent` (stale `self.Box.OnComponentBeginOverlap` _asbp_player)))
          (`PrimitiveComponent.SetCollisionEnabled` _capsulecomponent "NoCollision")
          (`PrimitiveComponent.SetCollisionEnabled` (`self.MainTable`) "NoCollision")
          (bind (_direction _newtrack_0) (`Timeline|CameraAnim` :!via `PlayFromStart`)
            (:`Update`
              (`self.SetPlayerPos` (`GameplayStatics.GetPlayerController` 0) _newtrack_0)
              (`PrimitiveComponent.SetCollisionEnabled` _capsulecomponent "QueryAndPhysics")
              (set `/Game/Blueprints/BP_player.IsSit` true (stale `self.Box.OnComponentBeginOverlap` _asbp_player))
              (if (`/Game/Blueprints/BP_player.IsSit` (stale `self.Box.OnComponentBeginOverlap` _asbp_player))
                (`SkeletalMeshComponent.PlayAnimation` (`Character.Mesh` (stale `self.Box.OnComponentBeginOverlap` _asbp_player)) "/Game/SimpleCrouchAnims/Animations/1Foot/AS_Crouch_1F_Idle.AS_Crouch_1F_Idle" true)
                (`Controller.SetIgnoreLookInput` _returnvalue false)
                (`KismetSystemLibrary.Delay` 5.0)
                (`Controller.ResetIgnoreLookInput` _returnvalue)))))))))

(event `Key|Q`
  (params (Key :type "Key Structure"))
  (:`Pressed`
    (bind _asbp_player (cast `/Game/Blueprints/BP_player` (stale `self.Box.OnComponentBeginOverlap` OtherActor)))
    (if (`/Game/Blueprints/BP_player.IsSit` (stale `self.Box.OnComponentBeginOverlap` _asbp_player))
      (set `/Game/Blueprints/BP_player.IsSit` false _asbp_player)
      (`SkeletalMeshComponent.SetAnimationMode` (`Character.Mesh` _asbp_player) "AnimationBlueprint"))))

(event `self.Box.OnComponentBeginOverlap`
  (params (OverlappedComponent :type "PrimitiveComponent Object Reference") (OtherActor :type "Actor Object Reference") (OtherComp :type "PrimitiveComponent Object Reference") (OtherBodyIndex :type Integer) (bFromSweep :type Boolean) (SweepResult :type "HitResult Structure (by ref)"))
  (set `self.Player` OtherActor)
  (`self.EnableInput` (`GameplayStatics.GetPlayerController` 0))
  (bind _asbp_player (cast `/Game/Blueprints/BP_player` OtherActor))
  (bind _returnvalue (`|CreateWidget` "/Game/SwitchCharacterWidget.SwitchCharacterWidget_C"))
  (`UserWidget.AddToViewport` _returnvalue 0)
  (goto _label :!via `Open`))

(event `Key|C`
  (params (Key :type "Key Structure"))
  (:`Pressed`
    (`self.K2_TeleportTo` :`self` (`self.Player`) :`DestLocation` (`self.K2_GetActorLocation` (`self.GodDesk`)))))

(event `self.Box.OnComponentEndOverlap`
  (params (OverlappedComponent :type "PrimitiveComponent Object Reference") (OtherActor :type "Actor Object Reference") (OtherComp :type "PrimitiveComponent Object Reference") (OtherBodyIndex :type Integer))
  (`Widget.RemoveFromParent` (stale `self.Box.OnComponentBeginOverlap` _returnvalue))
  (`self.DisableInput` (`GameplayStatics.GetPlayerController` 0))
  (goto _label :!via `Close`))

(fn `UserConstructionScript`)
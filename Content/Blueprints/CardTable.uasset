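; CardTable is an interactable actor that starts a Mountea dialogue with God when the player presses W nearby.
; Overlapping its Box enables the player controller's input on the actor and opens a Gate, while leaving disables input and closes it.
; A W press passing the Gate waits briefly, then initializes the dialogue with God as initiator and God's participant component as the dialogue participant.
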(event `Key|W`
  (params (Key :type "Key Structure"))
  (bind _god (`self.God`))
  (:`Pressed`
    (`/Engine/EditorBlueprintResources/StandardMacros.Gate` true :!label _label
      (:`Exit`
        (`KismetSystemLibrary.Delay` 1.0)
        (`MounteaDialogueSystemBFC.InitializeDialogue` _god (`/Game/Blueprints/GodTest.MounteaDialogueParticipant` _god))))))

(event `self.Box.OnComponentBeginOverlap`
  (params (OverlappedComponent :type "PrimitiveComponent Object Reference") (OtherActor :type "Actor Object Reference") (OtherComp :type "PrimitiveComponent Object Reference") (OtherBodyIndex :type Integer) (bFromSweep :type Boolean) (SweepResult :type "HitResult Structure (by ref)"))
  (`self.EnableInput` (`GameplayStatics.GetPlayerController` 0))
  (goto _label :!via `Open`))

(event `self.Box.OnComponentEndOverlap`
  (params (OverlappedComponent :type "PrimitiveComponent Object Reference") (OtherActor :type "Actor Object Reference") (OtherComp :type "PrimitiveComponent Object Reference") (OtherBodyIndex :type Integer))
  (`self.DisableInput` (`GameplayStatics.GetPlayerController` 0))
  (goto _label :!via `Close`))

(fn `UserConstructionScript`
  (`parent.UserConstructionScript`))
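; Player controller that switches input handling for Mountea dialogue and relays a skip button.
; When the dialogue manager's state becomes Active, it shows the cursor and sets UI-only input focused on the dialogue widget with the mouse locked.
; Other states hide the cursor and restore game-only input.
; Skip button press and release call the matching skip key events.
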(event `self.MounteaDialogueManager.OnDialogueManagerStateChanged`
  (params (NewState :type "EDialogueManagerState Enum (by ref)" :default "EDMS_Disabled"))
  (set `self.Show Mouse Cursor` (select `EDialogueManagerState` NewState :`EDMS_Active` true))
  (if (`self.Show Mouse Cursor`)
    (`WidgetBlueprintLibrary.SetInputMode_UIOnlyEx` self (`MounteaDialogueManager.GetDialogueUIPtr` (`self.MounteaDialogueManager`)) "LockAlways")
    (else
      (`WidgetBlueprintLibrary.SetInputMode_GameOnly` self))))

(event `InputAction|SkipButton`
  (params (Key :type "Key Structure"))
  (:`Pressed`
    (`self.SkipKeyPressed_Event`))
  (:`Released`
    (`self.SkipKeyReleased_Event`)))

(fn `UserConstructionScript`
  (`parent.UserConstructionScript`))